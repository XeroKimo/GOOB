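; Door frame actor that opens and closes moving doors by playing an assigned level sequence.
; Entering the box trigger plays the sequence forward, and leaving it plays the sequence in reverse.
; The IsStartingWingDoor flag changes this: flagged doors skip the reverse on exit, while unflagged doors also play the sequence at BeginPlay.
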(event `self.ReceiveBeginPlay`
  (if (not (`self.IsStartingWingDoor`))
    (`MovieSceneSequencePlayer.Play` (`LevelSequenceActor.SequencePlayer` (`self.SequenceToPlay`)))))

(event `self.Box.OnComponentBeginOverlap`
  (params (OverlappedComponent :type "PrimitiveComponent Object Reference") (OtherActor :type "Actor Object Reference") (OtherComp :type "PrimitiveComponent Object Reference") (OtherBodyIndex :type Integer) (bFromSweep :type Boolean) (SweepResult :type "HitResult Structure (by ref)"))
  (`MovieSceneSequencePlayer.Play` (`LevelSequenceActor.SequencePlayer` (`self.SequenceToPlay`))))

(event `self.Box.OnComponentEndOverlap`
  (params (OverlappedComponent :type "PrimitiveComponent Object Reference") (OtherActor :type "Actor Object Reference") (OtherComp :type "PrimitiveComponent Object Reference") (OtherBodyIndex :type Integer))
  (if (not (`self.IsStartingWingDoor`))
    (`MovieSceneSequencePlayer.PlayReverse` (`LevelSequenceActor.SequencePlayer` (`self.SequenceToPlay`)))))

(fn `UserConstructionScript`)